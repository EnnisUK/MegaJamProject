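; Interactable computer actor that the player toggles in and out of through its Interact event.
; Entering locks look input, blends the view to the computer, makes the Screen window focusable and, after the blend, enables the cursor and mouse click and hover events.
; Exiting blends back to the player character, then hides the cursor, restores look input and returns to game-only input.
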(event EventBeginPlay
  (bind _asplayer_bp (Utilities|Casting|CastToPlayer_BP (Game|GetPlayerCharacter 0)))
  (Variables|Default|SetAs%20Player%20BP _asplayer_bp))

(event Collision|EventActorBeginOverlap
  (params (OtherActor :type Actor%20Object%20Reference)))

(event EventTick
  (params (DeltaSeconds :type Float%20%28single-precision%29)))

(event EventInteract
  (bind _returnvalue (Game|GetPlayerController 0))
  (bind _returnvalue_2 (Game|GetPlayerController 0))
  (bind _returnvalue_3 (Game|GetPlayerController 0))
  (if (Variables|Default|GetIsInteracting?)
    (Game|Player|SetViewTargetwithBlend _returnvalue (Game|GetPlayerCharacter 0) 1.0 "VTBlend_Linear" 1.0 false)
    (Utilities|FlowControl|Delay 1.0)
    (Variables|/Script/Engine.PlayerController|SetbShowMouseCursor _returnvalue false)
    (Variables|Default|SetIsInteracting? false)
    (Input|SetIgnoreLookInput _returnvalue false)
    (Input|SetInputModeGameOnly _returnvalue false)
    (else
      (Input|SetIgnoreLookInput _returnvalue_2 true)
      (Class|WidgetComponent|SetWindowFocusable (Variables|Default|GetScreen) true)
      (Game|Player|SetViewTargetwithBlend _returnvalue_2 self 1.0 "VTBlend_Linear" 1.0 false)
      (Utilities|FlowControl|Delay 1.0)
      (Variables|/Script/Engine.PlayerController|SetbShowMouseCursor _returnvalue_2 true)
      (Variables|Default|SetIsInteracting? true)
      (Variables|/Script/Engine.PlayerController|SetbEnableClickEvents _returnvalue_3 true)
      (Variables|/Script/Engine.PlayerController|SetbEnableMouseOverEvents _returnvalue_3 true)
      (Input|EnableInput (Game|GetPlayerCharacter 0) _returnvalue_3))))

(fn ConstructionScript)