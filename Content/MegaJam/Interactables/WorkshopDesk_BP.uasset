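; Workshop desk pawn that the player can take control of and leave through interaction.
; On BeginPlay it caches the Player_BP character as the pawn to return to.
; Interact toggles IsAtTable, blending the camera to the desk or back to the player over one second, then possessing that pawn after a matching delay.
; The desk also handles the Interact input action by sending an Interact message.
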(event Input|EnhancedActionEvents|EnhancedInputActionInteract_Action
  (params (ActionValue :type Boolean) (ElapsedSeconds :type Float%20%28double-precision%29) (TriggeredSeconds :type Float%20%28double-precision%29) (InputAction :type Input%20Action%20Object%20Reference :default "/Game/MegaJam/Player/Inputs/Actions/Interact_Action.Interact_Action"))
  (:Triggered
    (Class|InteractBPI|Interact(Message) self)))

(event EventBeginPlay
  (bind _asplayer_bp (Utilities|Casting|CastToPlayer_BP (Game|GetPlayerCharacter 0))
    (:then
      (Variables|Default|SetAs%20Player%20BP _asplayer_bp)
      (Development|PrintString "Cast succ"))
    (:CastFailed
      (Development|PrintString "Cast Failed???"))))

(event Collision|EventActorBeginOverlap
  (params (OtherActor :type Actor%20Object%20Reference)))

(event EventTick
  (params (DeltaSeconds :type Float%20%28single-precision%29)))

(event EventInteract
  (bind _returnvalue (Game|GetPlayerController 0))
  (if (Variables|Default|GetIsAtTable?)
    (Development|PrintString "Posses Player")
    (Game|Player|SetViewTargetwithBlend (Game|GetPlayerController 0) (Variables|Default|GetAs%20Player%20BP) 1.0 "VTBlend_Linear" 0.0 false)
    (Utilities|FlowControl|Delay 1.0)
    (Variables|Default|SetIsAtTable? false)
    (Pawn|Possess _returnvalue (Variables|Default|GetAs%20Player%20BP))
    (else
      (Development|PrintString "Posses Table")
      (Game|Player|SetViewTargetwithBlend (Game|GetPlayerController 0) self 1.0 "VTBlend_Linear" 0.0 false)
      (Utilities|FlowControl|Delay 1.0)
      (Variables|Default|SetIsAtTable? true)
      (Pawn|Possess _returnvalue self))))

(fn ConstructionScript)